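; BP_APController is a controller Blueprint that exercises a custom HTTPObject by requesting hierarchy data from a hard-coded server.
; BeginPlay constructs the object, binds progress, completion and JSON callbacks, then executes the request.
; Progress and completion events print debug messages to screen.
; An auto-generated function receives a JSON callback struct and iterates its data without acting on it, so the response is not yet used.
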(event `self.ReceiveBeginPlay`
  (bind _returnvalue (`|GenericCreateObject` "/Script/Project_CPS.HTTPObject"))
  (set `self.BP_HTTPOB` _returnvalue)
  (add `HTTPObject.OnHttpConnectProcessCallback` _returnvalue (`|CreateDelegate` :!event `OnProceess`))
  (add `HTTPObject.OnHttpConnectFinishedCallback` _returnvalue (`|CreateDelegate` :!event `OnFinished`))
  (add `HTTPObject.JSonCallBack` _returnvalue (`|CreateDelegate` :!event `BP_APController_AutoGenFunc_Two`))
  (`HTTPObject.ExcuteHttp` (`self.BP_HTTPOB`) "http://133.186.215.97:51000" "/hierarchy/" "" ""))

(event `OnProceess`
  (params (RecvSize :type Integer) (TotalSize :type Integer) (Percent :type "Float (single-precision)"))
  (`KismetSystemLibrary.PrintString` (`KismetTextLibrary.Conv_TextToString` (`|FormatText` "{a}/{b} 는 {P}" RecvSize TotalSize Percent)) true true (struct :`R` 1.0 :`G` 0.095008 :`A` 1.0) 10.0))

(event `OnFinished`
  (params (bIsSuccess :type Boolean) (ContentPath :type String))
  (`KismetSystemLibrary.PrintString` (`KismetStringLibrary.Conv_BoolToString` bIsSuccess) true true (struct :`R` 1.0 :`G` 0.076702 :`A` 1.0) 10.0)
  (`KismetSystemLibrary.PrintString` "Hello"))

(fn `BP_APController_AutoGenFunc_Two`
  (params (Callbackstruct :type "StructArray Structure"))
  (set `self.Callbackstruct_two` Callbackstruct)
  (for _array_element (`.JsonData` (break `StructArray` Callbackstruct))
    _)
  (set `self.Array Element` _array_element)
  (return))

(fn `UserConstructionScript`)